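; AI controller for a patrolling guard NPC that tracks what it perceives.
; On BeginPlay it initializes the Patrol_BB blackboard and runs the GuardBehavior behavior tree.
; AI Perception updates write a successfully sensed actor into the EnemyActor key, with no filtering by actor type.
; A failed sense update clears that key, whichever actor triggered it.
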(event `self.ReceiveBeginPlay`
  (bind _blackboardcomponent (`self.UseBlackboard` "/Game/Dynamic/NPC/AI/Patrol_BB.Patrol_BB"))
  (set `self.BlackboardComp` _blackboardcomponent)
  (`self.RunBehaviorTree` "/Game/Dynamic/NPC/AI/GuardBehavior.GuardBehavior"))

(event `self.AIPerception.OnTargetPerceptionUpdated`
  (params (Actor :type "Actor Object Reference") (Stimulus :type "AIStimulus Structure"))
  (set `self.ActorSensed` Actor)
  (if (`.bSuccessfullySensed` (break `AIStimulus` Stimulus))
    (`BlackboardComponent.SetValueAsObject` (`self.BlackboardComp`) (`self.EnemyActor`) (`self.ActorSensed`))
    (else
      (`BlackboardComponent.ClearValue` (`self.BlackboardComp`) (`self.EnemyActor`)))))

(fn `UserConstructionScript`)